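; BP_AI is the DiscoBall enemy character, which detects, attacks and takes damage from the player.
; Pawn sensing sets a blackboard flag on seeing BP_Hero, and AttackPlayer sphere-traces forward to play a montage and damage the hero.
; A custom ApplyDamage event plays a hurt montage and subtracts fixed HP.
; Tick writes HP to the Health text, but its zero-HP check leads to no action.
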(event OnSeePawn(PawnSensing)
  (params (Pawn :type Pawn%20Object%20Reference))
  (Utilities|Casting|CastToBP_Hero Pawn)
  (AI|Components|Blackboard|SetValueasBool (AI|GetBlackboard (AI|GetAIController self)) (Utilities|Name|MakeLiteralName "hasSeenPlayer?") true))

(event Custom|Attack%20Player
  (bind _returnvalue (Transformation|GetActorLocation))
  (bind _outhit (Collision|SphereTraceForObjects _returnvalue (+ _returnvalue (* (Math|Vector|GetForwardVector (Transformation|GetActorRotation)) 2.5e+02) "") 1.2e+02 (Utilities|Array|MakeArray "ObjectTypeQuery3") false 0 "None"))
  (if true
    (Utilities|Casting|CastToBP_Hero (.HitActor (Collision|BreakHitResult _outhit)))
    (Animation|PlayAnimMontage "/Game/_MyFiles/Characters/DiscoBall/Animations/SKM_DiscoBall_Attack_Montage.SKM_DiscoBall_Attack_Montage" 1.0 "None")
    (Game|Damage|ApplyDamage (.HitActor (Collision|BreakHitResult _outhit)) 1e+01 0 0)))

(event EventBeginPlay)

(event Collision|EventActorBeginOverlap
  (params (OtherActor :type Actor%20Object%20Reference)))

(event EventApplyDamage
  (Animation|Montage|PlayMontage (Variables|Character|GetMesh) "/Game/_MyFiles/Characters/DiscoBall/Animations/SKM_DiscoBall_Damaged_Montage.SKM_DiscoBall_Damaged_Montage"
    (:then
      (Variables|Default|SetHP (- (Variables|Default|GetHP) 10)))))

(event EventTick
  (params (DeltaSeconds :type Float%20%28single-precision%29))
  (Rendering|Components|TextRender|SetText (Variables|Default|GetHealth) (Utilities|Text|ToText(Integer) (Variables|Default|GetHP)))
  (if (<= (Variables|Default|GetHP) 0)
    _))

(fn ConstructionScript)